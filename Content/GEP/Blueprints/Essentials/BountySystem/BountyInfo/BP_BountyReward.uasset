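; BP_BountyReward pays out a bounty's stat and item rewards to the player.
; It stores a parent bounty and the BP_PlayerCharacter found in the level, then reads reward lists from BountyInfo.
; Stat rewards add to Health, Mana or XP.
; Item rewards are Added to InventoryItems by name and count, but a unique item already held breaks the loop, skipping later items.
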(fn `GetParentBounty`
  (params (`Parent Bounty` :type "/Game/GEP/Blueprints/Essentials/BountySystem/BountyInfo/BP_Bounty Object Reference"))
  (set `self.Bounty` `Parent Bounty`))

(fn `GetPlayer`
  (bind _returnvalue (`GameplayStatics.GetActorOfClass` "/Game/GEP/Blueprints/Essentials/BP_PlayerCharacter.BP_PlayerCharacter_C"))
  (set `self.Player` _returnvalue))

(fn `GiveOutItemRewards`
  (bind _inventoryitems (`/Game/GEP/Blueprints/Essentials/BP_PlayerCharacter.InventoryItems` (`self.Player`)))
  (for _array_element (`.ItemRewards_23_080846EE4EFC73F5D8619CBF273D3752` (break `/Game/GEP/DataStructs/BountyDataTable` (`/Game/GEP/Blueprints/Essentials/BountySystem/BountyInfo/BP_Bounty.BountyInfo` (`self.Bounty`))))
    (bind (_itemname _count _isunique) (break `/Game/GEP/DataStructs/RewardItem` _array_element))
    (if _isunique
      (if (`BlueprintMapLibrary.Map_Contains` _inventoryitems _itemname)
        (break)
        (else
          _)))
    (`BlueprintMapLibrary.Map_Add` _inventoryitems _itemname _count)))

(fn `GiveOutStatRewards`
  (bind _player (`self.Player`))
  (for _array_element (`.StatRewards_20_228F7C904D763CA04259B2BA8ECB8BB5` (break `/Game/GEP/DataStructs/BountyDataTable` (`/Game/GEP/Blueprints/Essentials/BountySystem/BountyInfo/BP_Bounty.BountyInfo` (`self.Bounty`))))
    (bind (_statname _count) (break `/Game/GEP/DataStructs/RewardStat` _array_element))
    (switch `/Game/GEP/Blueprints/Essentials/E_PlayerInventory` _statname
      (:`NewEnumerator0`
        (set `/Game/GEP/Blueprints/Essentials/BP_PlayerCharacter.Health` (+ (`/Game/GEP/Blueprints/Essentials/BP_PlayerCharacter.Health` _player) _count) _player))
      (:`NewEnumerator1`
        (set `/Game/GEP/Blueprints/Essentials/BP_PlayerCharacter.Mana` (+ (`/Game/GEP/Blueprints/Essentials/BP_PlayerCharacter.Mana` _player) _count) _player))
      (:`NewEnumerator2`
        (set `/Game/GEP/Blueprints/Essentials/BP_PlayerCharacter.XP` (+ (`/Game/GEP/Blueprints/Essentials/BP_PlayerCharacter.XP` _player) _count) _player)))))