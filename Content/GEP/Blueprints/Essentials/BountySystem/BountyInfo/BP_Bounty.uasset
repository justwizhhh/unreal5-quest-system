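; BP_Bounty represents a single bounty, tracking its progress and handing out rewards.
; Init loads bounty info from a data table row, then links condition and reward components to itself, logging an error if the row is missing.
; While in progress, Tick has the condition component track conditions; deactivating clears progress.
; DistributeRewards gives stat and item rewards through the reward component and ends the bounty's progress state.
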(event `self.ReceiveTick`
  (params (DeltaSeconds :type "Float (single-precision)"))
  ;[0.05098 0.05098 0.05098] Updating the bounty's progress on the player (inside of BP_BountyCondition
  (if (`self.IsInProgress`)
    (`/Game/GEP/Blueprints/Essentials/BountySystem/BountyInfo/BP_BountyCondition.TrackConditions` (`self.BP_BountyCondition`))))

(event `Activate Bounty`
  (set `self.IsInProgress` true))

(event `Deactivate Bounty`
  (`/Game/GEP/Blueprints/Essentials/BountySystem/BountyInfo/BP_BountyCondition.ClearProgress` (`self.BP_BountyCondition`))
  (set `self.IsInProgress` false)
  (set `self.IsCompleted` false)
  (set `self.CurrentProgress` 0))

(fn `DistributeRewards`
  (bind _bp_bountyreward (`self.BP_BountyReward`))
  (`/Game/GEP/Blueprints/Essentials/BountySystem/BountyInfo/BP_BountyReward.GiveOutStatRewards` _bp_bountyreward)
  (`/Game/GEP/Blueprints/Essentials/BountySystem/BountyInfo/BP_BountyReward.GiveOutItemRewards` _bp_bountyreward)
  (set `self.IsInProgress` false))

(fn `Init`
  (bind _bp_bountyreward (`self.BP_BountyReward`))
  (bind _bp_bountycondition (`self.BP_BountyCondition`))
  ;[0.05098 0.05098 0.05098] Init - Making sure the bounty has at least one condition and at least one reward
  (bind _returnvalue (`|GetDataTableRow` "/Game/GEP/Bounties/GlobalBountyData.GlobalBountyData" (`self.BountyDataName`))
    (:`then`
      (set `self.BountyInfo` _returnvalue)
      (`/Game/GEP/Blueprints/Essentials/BountySystem/BountyInfo/BP_BountyCondition.GetParentBounty` _bp_bountycondition self)
      (`/Game/GEP/Blueprints/Essentials/BountySystem/BountyInfo/BP_BountyCondition.GenerateConditions` _bp_bountycondition)
      (`/Game/GEP/Blueprints/Essentials/BountySystem/BountyInfo/BP_BountyReward.GetParentBounty` _bp_bountyreward self)
      (`/Game/GEP/Blueprints/Essentials/BountySystem/BountyInfo/BP_BountyReward.GetPlayer` _bp_bountyreward))
    (:`RowNotFound`
      (`AutomationBlueprintFunctionLibrary.AddExpectedLogError` (`KismetStringLibrary.Concat_StrStr` "ERROR - No bounty info has been given to " (`KismetSystemLibrary.GetDisplayName` self))))))

(fn `UserConstructionScript`)