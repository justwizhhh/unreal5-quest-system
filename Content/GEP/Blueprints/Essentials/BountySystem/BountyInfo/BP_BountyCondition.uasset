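; Bounty condition tracker that records collect and explore progress for a parent bounty and decides when it is completed.
; GenerateConditions seeds per-item counts and per-location flags from BountyInfo; ClearProgress resets and rebuilds them.
; TrackConditions sums both tracker results into the bounty's CurrentProgress, completing it when the sum reaches the total condition count.
; Both trackers return at the first satisfied condition, so each contributes at most one.
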(fn `ClearProgress`
  (`BlueprintMapLibrary.Map_Clear` (`self.CollectProgress`))
  (`KismetArrayLibrary.Array_Clear` (`self.ExploreProgress`))
  (`self.GenerateConditions`)
  (set `self.ConditionsMet` 0))

(fn `GenerateConditions`
  (bind (_name _icon _description _collectconditions _exploreconditions) (break `/Game/GEP/DataStructs/BountyDataTable` (`/Game/GEP/Blueprints/Essentials/BountySystem/BountyInfo/BP_Bounty.BountyInfo` (`self.Bounty`))))
  ;[0.05098 0.05098 0.05098] Set up the tracking lists for every condition attached to this bounty
  (for _array_element _collectconditions
    (`BlueprintMapLibrary.Map_Add` (`self.CollectProgress`) (`.ObjectName_2_E9A7993D40C26BCD4D9460B410A87885` (break `/Game/GEP/DataStructs/ConditionCollect` _array_element))))
  (for _ _exploreconditions
    (`KismetArrayLibrary.Array_Add` (`self.ExploreProgress`))))

(fn `GetParentBounty`
  (params (ParentBounty :type "/Game/GEP/Blueprints/Essentials/BountySystem/BountyInfo/BP_Bounty Object Reference"))
  (set `self.Bounty` ParentBounty))

(fn `TrackCollectConditions`
  (returns (FinalProgress :type Integer))
  (locals (Progress :type Integer))
  (bind _collectprogress (`self.CollectProgress`))
  ;[1 1 1] Check if the player has every relevant item in their inventory for this bounty
  (set `local.Progress` 0)
  (if (!= (`BlueprintMapLibrary.Map_Length` _collectprogress) 0)
    (for _array_element (`.CollectConditions_18_D8B9F49043A50FBCEE93F2BB20B4E57A` (break `/Game/GEP/DataStructs/BountyDataTable` (`/Game/GEP/Blueprints/Essentials/BountySystem/BountyInfo/BP_Bounty.BountyInfo` (`self.Bounty`))))
      (bind _keys (`BlueprintMapLibrary.Map_Keys` _collectprogress))
      (for _ _keys
        (bind (_objectname _count) (break `/Game/GEP/DataStructs/ConditionCollect` _array_element))
        (bind (_value _returnvalue) (`BlueprintMapLibrary.Map_Find` _collectprogress _objectname))
        (if _returnvalue
          (if (>= _value _count)
            (bind _output_get (set `local.Progress` (+ (`local.Progress`) 1)))
            (return _output_get)))))))

(fn `TrackConditions`
  (bind _bounty (`self.Bounty`))
  (bind (_name _icon _description _collectconditions _exploreconditions) (break `/Game/GEP/DataStructs/BountyDataTable` (`/Game/GEP/Blueprints/Essentials/BountySystem/BountyInfo/BP_Bounty.BountyInfo` (`self.Bounty`))))
  (if (not (`/Game/GEP/Blueprints/Essentials/BountySystem/BountyInfo/BP_Bounty.IsCompleted` (`self.Bounty`)))
    (bind _finalprogress (`self.TrackCollectConditions`))
    (bind _finalprogress_2 (`self.TrackExploreConditions`))
    (bind _returnvalue (+ _finalprogress_2 _finalprogress))
    (bind _output_get (set `self.ConditionsMet` _returnvalue))
    (set `/Game/GEP/Blueprints/Essentials/BountySystem/BountyInfo/BP_Bounty.CurrentProgress` _output_get _bounty)
    (if (>= _returnvalue (+ (`KismetArrayLibrary.Array_Length` _collectconditions) (`KismetArrayLibrary.Array_Length` _exploreconditions)))
      (set `/Game/GEP/Blueprints/Essentials/BountySystem/BountyInfo/BP_Bounty.IsCompleted` true _bounty))))

(fn `TrackExploreConditions`
  (returns (FinalProgress :type Integer))
  (locals (Progress :type Integer))
  ;[0.05098 0.05098 0.05098] Check if the player has reached all target locations for this bounty
  (set `local.Progress` 0)
  (for _array_element (`self.ExploreProgress`)
    (if _array_element
      (bind _output_get (set `local.Progress` (+ (`local.Progress`) 1)))
      (return _output_get))))