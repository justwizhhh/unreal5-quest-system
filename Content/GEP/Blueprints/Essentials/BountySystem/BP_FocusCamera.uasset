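; BP_FocusCamera is a camera actor in the bounty system that animates a transition to a focus view and back.
; On BeginPlay it stores its camera's world transform as the end point.
; StartAnimation plays a timeline that lerps location and rotation from StartPos and StartRot, which are not set in this graph, to that end point.
; EndAnimation reverses the same timeline.
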(event `self.ReceiveBeginPlay`
  (bind _camera (`self.Camera`))
  ;[0.05098 0.05098 0.05098] Setting up start position of the camera
  (set `self.EndPos` (`SceneComponent.K2_GetComponentLocation` _camera))
  (set `self.EndRot` (`SceneComponent.K2_GetComponentRotation` _camera)))

(event `StartAnimation`
  (bind _camera (`self.Camera`))
  ;[0.05098 0.05098 0.05098] Playing fade-in and fade-out animations
  (bind (_direction _animationprogress) (`Timeline|Timeline` :!via `PlayFromStart` :!label _label)
    (:`Update`
      (`SceneComponent.K2_SetWorldLocation` _camera (`KismetMathLibrary.VLerp` (`self.StartPos`) (`self.EndPos`) _animationprogress) false false)
      (`SceneComponent.K2_SetWorldRotation` _camera (`KismetMathLibrary.RLerp` (`self.StartRot`) (`self.EndRot`) _animationprogress) false false))))

(event `EndAnimation`
  ;[0.05098 0.05098 0.05098] Playing fade-in and fade-out animations
  (goto _label :!via `ReverseFromEnd`))

(fn `UserConstructionScript`)